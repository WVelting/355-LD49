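; ComputerDesk is an interactable Blueprint that lets the player trade energy for progress on the GameDone stat.
; Its PlayerWantstoInteract event casts the first player controller to MyPlayerController, which holds all the stats it uses.
; While GameDone is below GameNeeded, each interaction raises GameDone and lowers Energy by fixed amounts, with no check on remaining Energy.
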(event `/Game/Blueprints/PlayerAndGame/Interfaces/PlayerCanInteract.Player Wants to Interact`
  (params (Player :type "/Game/Blueprints/PlayerAndGame/MainPlayer Object Reference"))
  (bind _asmy_player_controller (cast `/Game/Blueprints/PlayerAndGame/MyPlayerController` (`GameplayStatics.GetPlayerController` 0)))
  (bind _gamedone (`/Game/Blueprints/PlayerAndGame/MyPlayerController.GameDone` _asmy_player_controller))
  (if (< _gamedone (`/Game/Blueprints/PlayerAndGame/MyPlayerController.GameNeeded` _asmy_player_controller))
    (set `/Game/Blueprints/PlayerAndGame/MyPlayerController.GameDone` (+ _gamedone 10.0) _asmy_player_controller)
    (set `/Game/Blueprints/PlayerAndGame/MyPlayerController.Energy` (- (`/Game/Blueprints/PlayerAndGame/MyPlayerController.Energy` _asmy_player_controller) 25.0) _asmy_player_controller)))

(fn `UserConstructionScript`)