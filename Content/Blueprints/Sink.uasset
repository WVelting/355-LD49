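; Sink is an interactable Blueprint that lets the player do dishes at an energy cost.
; On PlayerWantstoInteract it casts the first player controller to MyPlayerController and checks whether DishesDone is still below DishesNeeded.
; If so, it increments DishesDone and subtracts a fixed amount of Energy directly on that controller, without checking how much energy remains.
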(event `/Game/Blueprints/PlayerAndGame/Interfaces/PlayerCanInteract.Player Wants to Interact`
  (params (Player :type "/Game/Blueprints/PlayerAndGame/MainPlayer Object Reference"))
  (bind _asmy_player_controller (cast `/Game/Blueprints/PlayerAndGame/MyPlayerController` (`GameplayStatics.GetPlayerController` 0)))
  (bind _dishesdone (`/Game/Blueprints/PlayerAndGame/MyPlayerController.DishesDone` _asmy_player_controller))
  (if (< _dishesdone (`/Game/Blueprints/PlayerAndGame/MyPlayerController.DishesNeeded` _asmy_player_controller))
    (set `/Game/Blueprints/PlayerAndGame/MyPlayerController.DishesDone` (+ _dishesdone 1.0) _asmy_player_controller)
    (set `/Game/Blueprints/PlayerAndGame/MyPlayerController.Energy` (- (`/Game/Blueprints/PlayerAndGame/MyPlayerController.Energy` _asmy_player_controller) 20.0) _asmy_player_controller)))

(fn `UserConstructionScript`)